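; SoundMaster_BP is a music visualizer actor that plays a sound and scales bar actors to match its frequency spectrum.
; The construction script gathers all AudioMaster_BP actors as bars, and BeginPlay starts the audio.
; Each playback-percent callback converts progress to seconds and samples precomputed, normalized Constant-Q data for channel 0.
; Each band value drives the cube height of the bar at the same array index.
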(event `self.ReceiveBeginPlay`
  (`AudioComponent.SetSound` (`self.Audio`) (`self.Sound`))
  (set `self.Duration` (`SoundBase.Duration` (`self.Sound`)))
  (add `AudioComponent.OnAudioPlaybackPercent` (`self.Audio`) (delegate `Playback`))
  (`AudioComponent.Play` (`self.Audio`) 0.0))

(event `Playback`
  (params (PlayingSoundWave :type "SoundWave Object Reference") (PlaybackPercent :type "Float (double-precision)"))
  (set `self.PlayedTime` (* PlaybackPercent (`self.Duration`)))
  (for (_array_element _array_index) (`ConstantQNRT.GetNormalizedChannelConstantQAtTime` (`self.Constant_REF`) (`self.PlayedTime`) 0)
    (bind _output (`|GetArrayItem` (`self.AudioBars`) _array_index))
    (`/Engine/EditorBlueprintResources/StandardMacros.IsValid` _output
      (:`Is Valid`
        (bind (_returnvalue_x _returnvalue_y _returnvalue_z) (`KismetMathLibrary.BreakVector` (* (`KismetMathLibrary.Conv_DoubleToVector` _array_element) 50.0)))
        (`SceneComponent.SetWorldScale3D` (`/Game/SoundVisualization/AudioMaster_BP.Cube` _output) (`KismetMathLibrary.MakeVector` 4.0 4.0 _returnvalue_z))))))

(fn `UserConstructionScript`
  (bind _outactors (`GameplayStatics.GetAllActorsOfClass` "/Game/SoundVisualization/AudioMaster_BP.AudioMaster_BP_C"))
  (set `self.AudioBars` _outactors))